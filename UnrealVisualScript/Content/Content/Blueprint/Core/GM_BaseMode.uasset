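; GM_BaseMode is the base game mode, handling player respawn, HUD creation, pause toggling and win/lose level transitions.
; It binds to the player's death and win-score dispatchers at BeginPlay, while respawning spawns and possesses a new BP_Player at a PlayerStart, rebinding only death.
; A seeded random stream is stepped up or down by events and reset with the quarter state on respawn.
; Tick prints the seed and quarter values for debugging.
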(event Custom|E_InitializeHUD
  (bind _returnvalue (UserInterface|CreateWidget "/Game/Content/Blueprint/Widget/WBP_HUD.WBP_HUD_C"))
  (UserInterface|Viewport|AddtoViewport _returnvalue 0))

(event EventBeginPlay
  (Utilities|FlowControl|Sequence
    (:then_0
      ;[0 0 0] Set Game Seed
      (Math|Random|SetRandomStreamSeed (Variables|Default|GetStream) 0))
    (:then_1
      ;[0 0 0] Bind Player Events
      (bind _asbp_player (Utilities|Casting|CastToBP_Player (Game|GetPlayerCharacter 0)))
      (EventDispatchers|BindEventtoEDPlayerDeath _asbp_player (EventDispatchers|CreateEvent :!event Custom|E_LooseScreen))
      (EventDispatchers|BindEventtoEDWinScore _asbp_player (EventDispatchers|CreateEvent :!event Custom|E_WinScreen)))))

(event EventTick
  (params (DeltaSeconds :type Float%20%28single-precision%29))
  ;[1 0 0] Seed State Debug
  (Development|PrintString (Utilities|String|Append (Utilities|String|ToString(Integer) (Variables|Default|GetStreamSeed)) "/////" (Utilities|String|ToString(Integer) (Variables|Default|GetCurrentQuarter)) "\\\\\\\\\\" (Utilities|String|ToString(Integer) (Variables|Default|GetPrecedentQuarter))) true true "(R=0.823201,G=1.000000,B=0.000000,A=1.000000)" 0.0))

(event Custom|E_SpawnPlayer
  ;[0 0.376 1] When the player pawn is destroyed, spawn a new pawn on a Player Start actor
  (bind _returnvalue (Actor|GetActorOfClass "/Script/Engine.PlayerStart"))
  (bind _returnvalue_2 (Game|SpawnActorfromClass "/Game/Content/Blueprint/Player/BP_Player.BP_Player_C" (Transformation|GetActorTransform _returnvalue) "Undefined" "MultiplyWithRoot" 0 0))
  (bind _output_get (Variables|Default|SetRef_PlayerActor _returnvalue_2))
  (Pawn|Possess (Game|GetPlayerController 0) _output_get)
  (EventDispatchers|BindEventtoEDPlayerDeath (Variables|Default|GetRef_PlayerActor) (EventDispatchers|CreateEvent :!event Custom|E_SpawnPlayer))
  ;[0 0 0] Reset Game Seed State
  (Math|Random|SetRandomStreamSeed (Variables|Default|GetStream) 0)
  (Variables|Default|SetStreamSeed 0)
  (Variables|Default|SetPrecedentQuarter 1)
  (Variables|Default|SetCurrentQuarter 1))

(event Custom|E_IncreaseSeed
  ;[0 0.376 1] Update Seed Value
  (bind _result (Math|Integer|IncrementInt (Variables|Default|GetStreamSeed))
    (:%20%20
      (Math|Random|SetRandomStreamSeed (Variables|Default|GetStream) _result))))

(event Custom|E_DecreSeed
  ;[0 0.376 1] Update Seed Value
  (bind _result (Math|Integer|DecrementInt (Variables|Default|GetStreamSeed))
    (:%20%20
      (Math|Random|SetRandomStreamSeed (Variables|Default|GetStream) _result))))

(event Custom|E_LooseScreen
  (Game|OpenLevel(byObjectReference) "/Game/Content/Level/L_LooseLevel.L_LooseLevel"))

(event Custom|E_WinScreen
  (Game|OpenLevel(byObjectReference) "/Game/Content/Level/L_WinLevel.L_WinLevel"))

(fn ConstructionScript)

(fn FHandlePauseRequest
  (bind _returnvalue (Game|GetPlayerController 0))
  (if (Game|IsGamePaused)
    (Game|SetGamePaused false)
    (Class|GameViewportSubsystem|RemoveWidget (|GameViewportSubsystem) (Variables|Default|GetPauseWidget))
    (Variables|/Script/Engine.PlayerController|SetbShowMouseCursor _returnvalue false)
    (Input|SetInputModeGameOnly _returnvalue false)
    (else
      (Game|SetGamePaused true)
      (Utilities|IsValid (Variables|Default|GetPauseWidget)
        (:Is%20Valid
          _)
        (:Is%20Not%20Valid
          (bind _returnvalue_2 (UserInterface|CreateWidget "/Game/Content/Blueprint/Widget/Menus/WBP_Pause.WBP_Pause_C"))
          (Variables|Default|SetPauseWidget _returnvalue_2)))
      (UserInterface|Viewport|AddtoViewport (Variables|Default|GetPauseWidget) 0))))