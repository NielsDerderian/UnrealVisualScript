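; Player character with Enhanced Input movement, health and a coffee-collection win condition.
; Input actions drive camera-relative movement, look, jump and a hold-to-walk speed switch.
; AnyDamage lowers health and updates a normalized UI value; at zero it stops movement, fires a death dispatcher and expires shortly after, though Died is set false.
; Added coffee accumulates until a threshold fires the win dispatcher; a debug key applies self-damage.
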(event Custom|E_InitializeHealth
  (bind _output_get (Variables|Settings|SetHealth (Variables|Settings|GetMaxHealth)))
  (Variables|Settings|SetUI_Health _output_get))

(event EventBeginPlay
  (bind _returnvalue (Game|GetPlayerController 0))
  (Utilities|FlowControl|Sequence
    (:then_0
      (CallFunction|EInitializeEnhancedInputs))
    (:then_1
      (CallFunction|EInitializeHealth))
    (:then_2
      (Variables|/Script/Engine.PlayerController|SetbShowMouseCursor _returnvalue false)
      (Input|SetInputModeGameOnly _returnvalue false))))

(event Game|Damage|EventAnyDamage
  (params (Damage :type Float%20%28single-precision%29) (DamageType :type Damage%20Type%20Object%20Reference) (InstigatedBy :type Controller%20Object%20Reference) (DamageCauser :type Actor%20Object%20Reference))
  (if (not (Variables|Settings|GetDied))
    (CallFunction|FResolveDamages Damage)))

(event Input|KeyboardEvents|DebugKeyF
  (params (Key :type Key%20Structure) (ActionValue :type Input%20Action%20Value%20Structure))
  (bind _self self)
  ;[1 0 0] Debug Self Damage
  (:Pressed
    (Game|Damage|ApplyDamage _self 1e+01 0 _self)))

(event Custom|E_InitializeEnhancedInputs
  (bind _asplayer_controller (Utilities|Casting|CastToPlayerController (Pawn|GetController)))
  (Utilities|IsValid (PlayerController|LocalPlayerSubsystems|GetEnhancedInputLocalPlayerSubsystem _asplayer_controller)
    (:Is%20Valid
      (Input|AddMappingContext (PlayerController|LocalPlayerSubsystems|GetEnhancedInputLocalPlayerSubsystem _asplayer_controller) "/Game/Content/Blueprint/Input/IMC_Default.IMC_Default" 0 "(bIgnoreAllPressedKeysUntilRelease=True,bForceImmediately=False)"))))

(event Input|EnhancedActionEvents|EnhancedInputActionIA_Walk
  (params (ActionValue :type Boolean) (ElapsedSeconds :type Float%20%28double-precision%29) (TriggeredSeconds :type Float%20%28double-precision%29) (InputAction :type Input%20Action%20Object%20Reference :default "/Game/Content/Blueprint/Input/Actions/IA_Walk.IA_Walk"))
  (bind _charactermovement (Variables|Character|GetCharacterMovement))
  (:Ongoing
    (Variables|/Script/Engine.CharacterMovementComponent|SetMaxWalkSpeed _charactermovement (Variables|Default|GetSpeed_Walk)))
  (:Canceled
    (Variables|/Script/Engine.CharacterMovementComponent|SetMaxWalkSpeed _charactermovement (Variables|Default|GetSpeed_Run) :!label _label))
  (:Completed
    (goto _label)))

(event Input|EnhancedActionEvents|EnhancedInputActionIA_Move
  (params (ActionValue :type Vector%202D%20Structure) (ElapsedSeconds :type Float%20%28double-precision%29) (TriggeredSeconds :type Float%20%28double-precision%29) (InputAction :type Input%20Action%20Object%20Reference :default "/Game/Content/Blueprint/Input/Actions/IA_Move.IA_Move"))
  (bind _returnvalue (Pawn|GetControlRotation :!class /Script/Engine.Pawn))
  (:Triggered
    (Variables|Default|SetPlayerStrafeDirection (.x ActionValue))
    (Variables|Default|SetPlayerMoveDirection (.y ActionValue))
    (Pawn|Input|AddMovementInput (Math|Vector|GetRightVector (Math|Rotator|MakeRotator (.roll _returnvalue) 0.0 (.yaw _returnvalue))) (.x ActionValue) false)
    (Pawn|Input|AddMovementInput (Math|Vector|GetForwardVector (Math|Rotator|MakeRotator 0.0 0.0 (.yaw (Pawn|GetControlRotation :!class /Script/Engine.Pawn)))) (.y ActionValue) false)))

(event Input|EnhancedActionEvents|EnhancedInputActionIA_Jump
  (params (ActionValue :type Boolean) (ElapsedSeconds :type Float%20%28double-precision%29) (TriggeredSeconds :type Float%20%28double-precision%29) (InputAction :type Input%20Action%20Object%20Reference :default "/Game/Content/Blueprint/Input/Actions/IA_Jump.IA_Jump"))
  (:Triggered
    (Character|Jump))
  (:Completed
    (Character|StopJumping)))

(event Input|EnhancedActionEvents|EnhancedInputActionIA_Look
  (params (ActionValue :type Vector%202D%20Structure) (ElapsedSeconds :type Float%20%28double-precision%29) (TriggeredSeconds :type Float%20%28double-precision%29) (InputAction :type Input%20Action%20Object%20Reference :default "/Game/Content/Blueprint/Input/Actions/IA_Look.IA_Look"))
  (:Triggered
    (Pawn|Input|AddControllerYawInput (.x ActionValue))
    (Pawn|Input|AddControllerPitchInput (.y ActionValue))))

(fn ConstructionScript)

(fn FResolveDamages
  (params (DamageTaken :type Float%20%28double-precision%29))
  (bind _self self)
  (bind _output_get (Variables|Settings|SetHealth (Math|Float|Clamp(Float) (- (Variables|Settings|GetHealth) DamageTaken) 0.0 1e+02)))
  (Variables|Settings|SetUI_Health (Math|Float|Clamp(Float) (/ _output_get (Variables|Settings|GetMaxHealth))))
  (if (<= (Variables|Settings|GetHealth) 0.0)
    (CallFunction|FKillPlayer)
    (elif (< DamageTaken 0.0)
      (CallFunction|HPrint (Utilities|String|ToString(Float) (Variables|Settings|GetHealth)) "(R=0.786458,G=0.000000,B=0.000000,A=1.000000)" 1.0 _self)
      (else
        (CallFunction|HPrint (Utilities|String|ToString(Float) (Variables|Settings|GetHealth)) "(R=0.072184,G=0.661458,B=0.000000,A=1.000000)" 1.0 _self)))))

(fn FKillPlayer
  (Components|Movement|StopMovementImmediately (Variables|Character|GetCharacterMovement))
  (Variables|Settings|SetDied false)
  (Actor|SetLifeSpan 0.2)
  (Default|CallEDPlayerDeath))

(fn FAddCoffee
  (params (CoffeeToAdd :type Integer) (FromCoffee :type Boolean))
  (bind _output_get (Variables|Default|SetCoffeeAmount (+ CoffeeToAdd (Variables|Default|GetCoffeeAmount))))
  (if (>= _output_get 10)
    (Default|CallEDWinScore)
    (else
      (return _output_get))))