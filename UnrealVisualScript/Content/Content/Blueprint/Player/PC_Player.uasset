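; Player controller that builds the HUD and forwards pause input to the base game mode.
; On BeginPlay it caches the GM_BaseMode reference and binds E_LoadHUD to a load-HUD event dispatcher, which creates WBP_HUD and adds it to the viewport when fired.
; The IA_Pause Enhanced Input action calls the game mode's pause request handler, leaving pause logic to the mode.
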(event Custom|E_LoadHUD
  (bind _returnvalue (UserInterface|CreateWidget "/Game/Content/Blueprint/Widget/WBP_HUD.WBP_HUD_C"))
  (UserInterface|Viewport|AddtoViewport _returnvalue 0))

(event Input|EnhancedActionEvents|EnhancedInputActionIA_Pause
  (params (ActionValue :type Boolean) (ElapsedSeconds :type Float%20%28double-precision%29) (TriggeredSeconds :type Float%20%28double-precision%29) (InputAction :type Input%20Action%20Object%20Reference :default "/Game/Content/Blueprint/Input/Actions/IA_Pause.IA_Pause"))
  (:Started
    (Default|FHandlePauseRequest (Variables|Default|GetAs%20GM%20Base%20Mode))))

(event EventBeginPlay
  (Utilities|FlowControl|Sequence
    (:then_0
      (bind _asgm_base_mode (Utilities|Casting|CastToGM_BaseMode (Game|GetGameMode)))
      (Variables|Default|SetAs%20GM%20Base%20Mode _asgm_base_mode))
    (:then_1
      (EventDispatchers|BindEventtoEDLoadHUD (delegate Custom|E_LoadHUD)))))

(fn ConstructionScript)