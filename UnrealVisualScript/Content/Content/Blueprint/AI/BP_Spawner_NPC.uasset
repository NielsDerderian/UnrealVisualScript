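; BP_Spawner_NPC is an actor that spawns NPCs around itself when play begins.
; It loops up to the shortfall between NumbertoSpawn and NpcAlive, using each index as a DT_NPCs row name to pick the class.
; Each found row spawns at a random navigable point within a fixed radius, with random yaw.
; Spawned actors join AliveNPCs, and NpcAlive is then set to that array's length minus one.
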(event Custom|E_Spawn%20NPC
  (for _index (range 0 (CallFunction|FNPCtoSpawn))
    (bind _returnvalue (Utilities|GetDataTableRow "/Game/Content/Blueprint/AI/NPCs/DT_NPCs.DT_NPCs" (Utilities|String|StringToName (Utilities|String|ToString(Integer) _index)))
      (:then
        (bind _randomlocation (Class|NavigationSystemV1|GetRandomLocationinNavigableRadius (Transformation|GetActorLocation) 2.4e+03 0 0))
        (bind _returnvalue_2 (Game|SpawnActorfromClass (Utilities|Struct|BreakStruct_Npcs _returnvalue) (Math|Transform|MakeTransform _randomlocation (Math|Rotator|MakeRotator 0.0 0.0 (.Yaw (Math|Rotator|BreakRotator (Math|Random|RandomRotator false)))) "1.000000,1.000000,1.000000") "Undefined" "MultiplyWithRoot" 0 0))
        (Utilities|Array|Add (Variables|Default|GetAliveNPCs) _returnvalue_2))))
  (Variables|Default|SetNpcAlive (- (Utilities|Array|Length (Variables|Default|GetAliveNPCs)) 1)))

(event EventBeginPlay
  (CallFunction|ESpawnNPC))

(fn ConstructionScript)

(fn FNPCtoSpawn
  (return (- (Variables|Default|GetNumbertoSpawn) (Variables|Default|GetNpcAlive))))