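; AI controller for NPCs that runs the BT_NPC behavior tree and feeds it player detection from AI perception.
; Sensing an actor tagged Player cancels the lose-sight timer and writes line of sight and the target actor to the blackboard.
; Any other perception update starts a one-shot timer of LooseSightTimer length, which clears both keys when it fires.
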(event OnTargetPerceptionUpdated(AIPerception)
  (params (Actor :type Actor%20Object%20Reference) (Stimulus :type AI%20Stimulus%20Structure))
  (if (and (Actor|ActorHasTag Actor "Player") (Utilities|Struct|BreakAIStimulus Stimulus))
    (Utilities|Time|ClearandInvalidateTimerbyHandle (Variables|Default|GetTimer_Sight))
    (CallFunction|FUpdateSightKey true)
    (CallFunction|FUpdateTargetActorKey Actor)
    (else
      (bind _returnvalue (Utilities|Time|SetTimerbyEvent (delegate Custom|StartSightTimer) (Variables|Default|GetLooseSightTimer)))
      (Variables|Default|SetTimer_Sight _returnvalue))))

(event Custom|StartSightTimer
  (CallFunction|FUpdateSightKey false)
  (CallFunction|FUpdateTargetActorKey))

(event EventBeginPlay
  (AI|RunBehaviorTree "/Game/Content/Blueprint/AI/BT_NPC.BT_NPC"))

(fn ConstructionScript)

(fn FUpdateSightKey
  (params (HasLineOfSight :type Boolean))
  (AI|Components|Blackboard|SetValueasBool (Variables|Default|GetBlackboard) (Variables|Default|GetHasLineOfSight) HasLineOfSight))

(fn FUpdateTargetActorKey
  (params (TargetedActor :type Object%20Object%20Reference))
  (AI|Components|Blackboard|SetValueasObject (Variables|Default|GetBlackboard) (Variables|Default|GetPlayerActor) TargetedActor))