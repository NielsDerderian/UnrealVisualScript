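; BP_Collectables is a pickup that gives coffee to the player on contact.
; When BP_Player overlaps its sphere collider, it plays a loot sound at its location, calls FAddCoffee on the player and destroys itself.
; The construction script randomizes the RotatingMovement yaw rate and the InterpToMovement vertical control points, giving each instance its own spin and bob range.
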(event OnComponentBeginOverlap(Sphere_Collider)
  (params (OverlappedComponent :type Primitive%20Component%20Object%20Reference) (OtherActor :type Actor%20Object%20Reference) (OtherComp :type Primitive%20Component%20Object%20Reference) (OtherBodyIndex :type Integer) (bFromSweep :type Boolean) (SweepResult :type Hit%20Result%20Structure%20%28by%20ref%29))
  (bind _asbp_player (Utilities|Casting|CastToBP_Player OtherActor))
  (Audio|PlaySoundatLocation (Variables|Default|GetLootSound) (Transformation|GetActorLocation) "0, 0, 0" 1.0 1.0 0.0 0 0 0 0)
  (Default|FAddCoffee _asbp_player (Variables|Default|GetCoffee%20to%20Add) true)
  (Actor|DestroyActor))

(event EventBeginPlay)

(event Collision|EventActorBeginOverlap
  (params (OtherActor :type Actor%20Object%20Reference)))

(event EventTick
  (params (DeltaSeconds :type Float%20%28single-precision%29)))

(fn ConstructionScript
  (Variables|/Script/Engine.RotatingMovementComponent|SetRotationRate (Variables|Default|GetRotatingMovement) (Math|Rotator|MakeRotator 0.0 0.0 (Math|Random|RandomFloatinRange 3e+01 1e+02)))
  (Variables|/Script/Engine.InterpToMovementComponent|SetControlPoints (Variables|Default|GetInterpToMovement) (Utilities|Array|MakeArray (Utilities|Struct|MakeInterpControlPoint (Math|Vector|MakeVector 0.0 0.0 (Math|Random|RandomFloatinRange -1e+01 0.0)) true) (Utilities|Struct|MakeInterpControlPoint (Math|Vector|MakeVector 0.0 0.0 (Math|Random|RandomFloatinRange 5.0 2e+01)) true))))