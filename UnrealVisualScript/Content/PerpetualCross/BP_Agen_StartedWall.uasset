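; BP_Agen_StartedWall is a wall actor that appears or vanishes when the PerpetualCross level regenerates.
; Its ERegen event shows the Cube with full collision when the game mode's StreamSeed is 0, or when PrecedentQuarter is 4 and StreamSeed is 2.
; Otherwise it hides the Cube and disables its collision.
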(event EventBeginPlay
  (|CallParentFunction) ; This node is disabled and will not be called.\nDrag off pins to build functionality.
)

(event EventERegen
  (bind _cube (Variables|Default|GetCube))
  (bind _cube_2 (Variables|Default|GetCube))
  (bind _as_gm_base_mode (Variables|Default|GetAs%20GM%20Base%20Mode))
  (if (or (== (Variables|/Game/Content/Blueprint/Core/GM_BaseMode.GM_BaseMode_C|GetStreamSeed (Variables|Default|GetAs%20GM%20Base%20Mode)) 0) (and (== (Variables|/Game/Content/Blueprint/Core/GM_BaseMode.GM_BaseMode_C|GetPrecedentQuarter _as_gm_base_mode) 4) (== (Variables|/Game/Content/Blueprint/Core/GM_BaseMode.GM_BaseMode_C|GetStreamSeed _as_gm_base_mode) 2)))
    (Rendering|SetVisibility _cube true false)
    (Collision|SetCollisionEnabled _cube "QueryAndPhysics")
    (else
      (Rendering|SetVisibility _cube_2 false false)
      (Collision|SetCollisionEnabled _cube_2 "NoCollision"))))

(fn ConstructionScript
  (|CallParentFunction))