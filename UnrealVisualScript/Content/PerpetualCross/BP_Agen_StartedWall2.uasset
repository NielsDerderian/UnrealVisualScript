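; BP_Agen_StartedWall2 is a level arrangement piece that shows or hides a wall depending on the game mode's current stream seed.
; On regeneration, after a short delay, it checks StreamSeed and PrecedentQuarter to toggle visibility and collision on SMAgen and StaticMesh.
; SMAgen returns to its cached start location when shown and moves to world origin when hidden, avoiding per-instance collision removal on the ISM.
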(event EventBeginPlay
  (|CallParentFunction)
  (Variables|Default|SetInitialLocation (Transformation|GetWorldLocation (Variables|Default|GetSM_Agen))))

(event EventERegen
  (bind _sm_agen (Variables|Default|GetSM_Agen))
  (bind _as_gm_base_mode (Variables|Default|GetAs%20GM%20Base%20Mode))
  (Utilities|FlowControl|Delay 0.2)
  (if (or (== (Variables|/Game/Content/Blueprint/Core/GM_BaseMode.GM_BaseMode_C|GetStreamSeed (Variables|Default|GetAs%20GM%20Base%20Mode)) 0) (and (== (Variables|/Game/Content/Blueprint/Core/GM_BaseMode.GM_BaseMode_C|GetPrecedentQuarter _as_gm_base_mode) 4) (== (Variables|/Game/Content/Blueprint/Core/GM_BaseMode.GM_BaseMode_C|GetStreamSeed _as_gm_base_mode) 2)))
    ;[0 0 0] Moving the ISM to not have to remove their collisions 1 by 1
    (Rendering|SetVisibility _sm_agen true true)
    (Collision|SetCollisionEnabled _sm_agen "QueryAndPhysics")
    (Transformation|SetWorldLocation _sm_agen (Variables|Default|GetInitialLocation) false false)
    (else
      (Rendering|SetVisibility _sm_agen false true)
      (Collision|SetCollisionEnabled _sm_agen "NoCollision")
      (Transformation|SetWorldLocation _sm_agen "0, 0, 0" false false))))

(fn ConstructionScript
  (|CallParentFunction))