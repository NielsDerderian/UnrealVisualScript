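; BP_Agen is an actor that displays a randomly chosen static mesh on its SMAgen component.
; Shortly after BeginPlay it caches GM_BaseMode and runs E_Regen, which picks from the AgenMesh array using the game mode's random stream, so the choice follows the seed.
; F_SetAgentList lets the mesh array be supplied from outside.
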(event Custom|E_Regen
  ;[0 0 0] Random Mesh From Seed
  (Components|StaticMesh|SetStaticMesh (Variables|Default|GetSM_Agen) (.OutItem (Utilities|Array|RandomFromStream (Variables|Default|GetAgenMesh) (Variables|/Game/Content/Blueprint/Core/GM_BaseMode.GM_BaseMode_C|GetStream (Variables|Default|GetAs%20GM%20Base%20Mode))))))

(event EventBeginPlay
  (bind _asgm_base_mode (Utilities|Casting|CastToGM_BaseMode (Game|GetGameMode)))
  (Variables|Default|SetAs%20GM%20Base%20Mode _asgm_base_mode)
  (Utilities|FlowControl|Delay 0.1)
  (CallFunction|ERegen))

(fn ConstructionScript)

(fn FSetAgentList
  (params (AgenMesh :type Array%20of%20Static%20Mesh%20Object%20References))
  (Variables|Default|SetAgenMesh AgenMesh))