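; BP_Quarter is a trigger volume for one numbered quarter of a loop that changes the world seed as the player moves between quarters.
; On player overlap, it shifts current and previous quarter IDs in GM_BaseMode and compares them for direction, treating 1 and 4 as neighbours.
; It then increases or decreases the game mode's seed, with same-quarter re-entry counting as a decrease, and regenerates BP_Agen actors found by QuarterTag.
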(event OnComponentBeginOverlap(QuarterBox)
  (params (OverlappedComponent :type Primitive%20Component%20Object%20Reference) (OtherActor :type Actor%20Object%20Reference) (OtherComp :type Primitive%20Component%20Object%20Reference) (OtherBodyIndex :type Integer) (bFromSweep :type Boolean) (SweepResult :type Hit%20Result%20Structure%20%28by%20ref%29))
  (bind _as_gm_base_mode (Variables|Default|GetAs%20GM%20Base%20Mode))
  (bind _as_gm_base_mode_2 (Variables|Default|GetAs%20GM%20Base%20Mode))
  (bind _as_gm_base_mode_3 (Variables|Default|GetAs%20GM%20Base%20Mode))
  (bind _as_gm_base_mode_4 (Variables|Default|GetAs%20GM%20Base%20Mode))
  (Utilities|Casting|CastToBP_Player OtherActor)
  (Variables|/Game/Content/Blueprint/Core/GM_BaseMode.GM_BaseMode_C|SetPrecedentQuarter _as_gm_base_mode_4 (Variables|/Game/Content/Blueprint/Core/GM_BaseMode.GM_BaseMode_C|GetCurrentQuarter _as_gm_base_mode_4))
  (bind _output_get (Variables|/Game/Content/Blueprint/Core/GM_BaseMode.GM_BaseMode_C|SetCurrentQuarter _as_gm_base_mode_3 (Variables|Default|GetID)))
  (if (> _output_get (Variables|/Game/Content/Blueprint/Core/GM_BaseMode.GM_BaseMode_C|GetPrecedentQuarter _as_gm_base_mode_3))
    (if (and (== _output_get 4) (== (Variables|/Game/Content/Blueprint/Core/GM_BaseMode.GM_BaseMode_C|GetPrecedentQuarter _as_gm_base_mode_3) 1))
      (Default|EDecreSeed (Variables|Default|GetAs%20GM%20Base%20Mode) :!label _label)
      (bind _outactors (Actor|GetAllActorswithTag (Variables|Default|GetQuarterTag)))
      (for _array_element _outactors
        (bind _asbp_agen (Utilities|Casting|CastToBP_Agen _array_element))
        (Default|ERegen _asbp_agen))
      (if (not (<= (Variables|/Game/Content/Blueprint/Core/GM_BaseMode.GM_BaseMode_C|GetPrecedentQuarter _as_gm_base_mode_2) 3))
        (bind _output_get_2 (Variables|/Game/Content/Blueprint/Core/GM_BaseMode.GM_BaseMode_C|SetPrecedentQuarter _as_gm_base_mode_2 4))
        (Development|PrintString (Utilities|String|ToString(Integer) _output_get_2) true true "(R=1.000000,G=0.000000,B=0.116688,A=1.000000)"))
      (else
        (Default|EIncreaseSeed (Variables|Default|GetAs%20GM%20Base%20Mode) :!label _label_2)
        (bind _outactors_2 (Actor|GetAllActorswithTag (Variables|Default|GetQuarterTag)))
        (for _array_element_2 _outactors_2
          (bind _asbp_agen_2 (Utilities|Casting|CastToBP_Agen _array_element_2))
          (Default|ERegen _asbp_agen_2))
        (if (not (>= (Variables|/Game/Content/Blueprint/Core/GM_BaseMode.GM_BaseMode_C|GetPrecedentQuarter _as_gm_base_mode) 1))
          (bind _output_get_3 (Variables|/Game/Content/Blueprint/Core/GM_BaseMode.GM_BaseMode_C|SetPrecedentQuarter _as_gm_base_mode 1))
          (Development|PrintString (Utilities|String|ToString(Integer) _output_get_3) true true "(R=0.000000,G=1.000000,B=0.008637,A=1.000000)"))))
    (elif (and (== _output_get 1) (== (Variables|/Game/Content/Blueprint/Core/GM_BaseMode.GM_BaseMode_C|GetPrecedentQuarter _as_gm_base_mode_3) 4))
      (goto _label_2)
      (else
        (goto _label)))))

(event EventBeginPlay
  (bind _asgm_base_mode (Utilities|Casting|CastToGM_BaseMode (Game|GetGameMode)))
  (Variables|Default|SetAs%20GM%20Base%20Mode _asgm_base_mode))

(fn ConstructionScript)